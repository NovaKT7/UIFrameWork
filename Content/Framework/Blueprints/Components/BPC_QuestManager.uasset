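; Player-owned component that tracks a list of quests and their progress through the actors each quest watches.
; AddQuest stores and announces a quest, then activates and binds to each watched actor's BPC_QuestComponent.
; QuestUpdated recalculates progress as the completed fraction of objectives, counting missing actors or components as complete.
; It saves the result, prints status, and broadcasts update and completion events for UI or other listeners.
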(event `self.ReceiveBeginPlay`
  (bind _asbp_base_player (cast `/Game/Framework/Blueprints/Characters/BP_BasePlayer` (`self.GetOwner`)))
  (set `self.Player` _asbp_base_player))

(event `QuestUpdated`
  (params (ID :type String))
  (for (_array_element _array_index) (`self.QuestList`)
    (bind ((`ID_13_2413B8D443A079090AB1D889FCC0CC71` _id) (`Complete_19_F04DF05F4D535DC695C4F3A5CDF8C141` _complete)) (break `/Game/Framework/Blueprints/Quest/sQuest` _array_element))
    (if _complete
      _
      (elif (`KismetStringLibrary.EqualEqual_StrStr` _id ID)
        (bind (_progress _outarray) (`self.CalcProgress` (`.ActorsToWatch_26_16E27CAB46EB0C0FD1A86F9CAA0B1D05` (break `/Game/Framework/Blueprints/Quest/sQuest` _array_element))))
        (bind _returnvalue (>= _progress 1.0))
        (bind _structout (setmembers `/Game/Framework/Blueprints/Quest/sQuest` :`StructRef` _array_element :`Actors To Watch` _outarray :`Progress` _progress :`Complete` _returnvalue))
        (`KismetArrayLibrary.Array_Set` (`self.QuestList`) _array_index _structout)
        (bind (_id_2 _questname _questdescription _icon _type _actorstowatch _progress_2 _complete_2) (break `/Game/Framework/Blueprints/Quest/sQuest` _structout))
        (`KismetSystemLibrary.PrintText` (`|FormatText` "{Quest Name} - Progress: {x}, status: {stat}" _questname _progress_2 (`KismetMathLibrary.SelectString` "Complete" "In Progress" _complete_2)) true true (struct :`R` 1.0 :`G` 0.14678 :`A` 1.0))
        (`self.OnQuestUpdated` _structout)
        (if _returnvalue
          (`self.OnQuestComplete` _structout))))))

(fn `AddQuest`
  (params (NewQuest :type "/Game/Framework/Blueprints/Quest/sQuest Structure"))
  (bind (_id _questname _questdescription _icon _type _actorstowatch) (break `/Game/Framework/Blueprints/Quest/sQuest` (`local.NewQuest`)))
  (`KismetArrayLibrary.Array_Add` (`self.QuestList`) NewQuest)
  (`self.OnQuestAdded` NewQuest (`self.Player`))
  (for _array_element _actorstowatch
    (bind _returnvalue (`Actor.GetComponentByClass` (`.ActorToWatch_8_A0799E1242B4B7F82E2A239D43189D95` (break `/Game/Framework/Blueprints/Quest/sObjective` _array_element)) "/Game/Framework/Blueprints/Quest/BPC_QuestComponent.BPC_QuestComponent_C"))
    (`/Game/Framework/Blueprints/Quest/BPC_QuestComponent.ActivateQuest` _returnvalue _id)
    (add `/Game/Framework/Blueprints/Quest/BPC_QuestComponent.OnQuestCompleted` _returnvalue (`|CreateDelegate` :!event `QuestUpdated`))))

(fn `CalcProgress`
  (params (ObjectiveArray :type "Array of /Game/Framework/Blueprints/Quest/sObjective Structure"))
  (returns (Progress :type "Float (double-precision)") (OutArray :type "Array of /Game/Framework/Blueprints/Quest/sObjective Structure"))
  (locals (ObjCount :type Integer :default 0) (Complete :type Integer) (L_Index :type Integer) (Objectives :type "Array of /Game/Framework/Blueprints/Quest/sObjective Structure"))
  (set `local.Objectives` ObjectiveArray)
  (set `local.ObjCount` (`KismetArrayLibrary.Array_Length` ObjectiveArray))
  (for (_array_element _array_index) (`local.Objectives`)
    (set `local.L_Index` _array_index)
    (bind (_objectivetitle _objectivedescription _icon _actortowatch _complete) (break `/Game/Framework/Blueprints/Quest/sObjective` _array_element))
    (if _complete
      (`/Engine/EditorBlueprintResources/StandardMacros.IncrementInt` (`local.Complete`))
      (else
        (`/Engine/EditorBlueprintResources/StandardMacros.IsValid` _actortowatch
          (:`Is Valid`
            (bind _returnvalue (`Actor.GetComponentByClass` _actortowatch "/Game/Framework/Blueprints/Quest/BPC_QuestComponent.BPC_QuestComponent_C"))
            (`/Engine/EditorBlueprintResources/StandardMacros.IsValid` _returnvalue
              (:`Is Valid`
                (bind _iscomplete (`/Game/Framework/Blueprints/Quest/BPC_QuestComponent.IsComplete` _returnvalue))
                (bind _structout (setmembers `/Game/Framework/Blueprints/Quest/sObjective` :`StructRef` (`|GetArrayItem` (`local.Objectives`) (`local.L_Index`)) :`Complete` _iscomplete))
                (`KismetArrayLibrary.Array_Set` (`local.Objectives`) (`local.L_Index`) _structout)
                (if _iscomplete
                  (`/Engine/EditorBlueprintResources/StandardMacros.IncrementInt` (`local.Complete`))))
              (:`Is Not Valid`
                (`/Engine/EditorBlueprintResources/StandardMacros.IncrementInt` (`local.Complete`) :!label _label))))
          (:`Is Not Valid`
            (goto _label))))))
  (return (/ (`local.Complete`) (`local.ObjCount`))))