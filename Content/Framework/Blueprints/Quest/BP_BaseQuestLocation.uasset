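; BP_BaseQuestLocation is a base quest location actor that the player completes by walking into it.
; Its quest mesh stays hidden until the quest component activates, which also shows the mesh and initializes a minimap POI marker.
; A player-tagged overlap on the collision box asks the quest component to complete the quest and, on success, destroys the actor.
; An older InitialisePOI event is kept but marked deprecated.
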(event `self.ReceiveBeginPlay`
  (`SceneComponent.SetVisibility` (`self.QuestMesh`) false false))

(event `self.BPC_QuestComponent.OnQuestActivated`
  (params (Comp :type "/Game/Framework/Blueprints/Quest/BPC_QuestComponent Object Reference"))
  (`/Game/Framework/Blueprints/Components/BPC_MinimapPOI.Init_QuestMarker` (`self.BPC_MinimapPOI`))
  (`SceneComponent.SetVisibility` (`self.QuestMesh`) true false))

(event `/Game/Framework/Blueprints/Interfaces/BPI_Minimap.InitialisePOI`
  (params (ModeRef :type "/Game/Framework/Blueprints/Modes/BP_RPGMode Object Reference"))
  ;[1 1 1] Deprecated
  (message `/Game/Framework/Blueprints/Interfaces/BPI_Minimap.InitialisePOI` (`self.BPC_MinimapPOI`) ModeRef))

(event `self.CollisionBox.OnComponentBeginOverlap`
  (params (OverlappedComponent :type "PrimitiveComponent Object Reference") (OtherActor :type "Actor Object Reference") (OtherComp :type "PrimitiveComponent Object Reference") (OtherBodyIndex :type Integer) (bFromSweep :type Boolean) (SweepResult :type "HitResult Structure (by ref)"))
  (if (`self.ActorHasTag` OtherActor "Player")
    (bind _success (`/Game/Framework/Blueprints/Quest/BPC_QuestComponent.CompleteQuest` (`self.BPC_QuestComponent`)))
    (if _success
      (`self.RemoveEffect`))))

(event `RemoveEffect`
  (`self.K2_DestroyActor`))

(fn `UserConstructionScript`)