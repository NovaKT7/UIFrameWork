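; Quest component that tracks one quest's ID and completion state on its owner.
; ActivateQuest stores the ID, activates the component and fires OnQuestActivated with itself.
; CompleteQuest only succeeds while the component is active, setting IsComplete, firing OnQuestCompleted with the ID, and returning success and ID.
; Component activation doubles as the quest's active flag; completing it does not deactivate the component.
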(event `ActivateQuest`
  (params (ID :type String))
  (set `self.ID` ID)
  (`self.Activate` false)
  (`self.OnQuestActivated` self))

(fn `CompleteQuest`
  (returns (Success :type Boolean) (ID :type String))
  (if (`self.IsActive`)
    (set `self.IsComplete` true)
    (`self.OnQuestCompleted` (`self.ID`))
    (return true (`self.ID`))
    (else
      (return false (`self.ID`)))))